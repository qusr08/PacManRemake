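; BP_Grid is the tile map for a Pac-Man-style Paper2D maze, storing walls, pellets and power pellets in a flat cell array.
; On BeginPlay it clears the grid, then snaps Paper Sprite actors that have a BP_GridComponent to 16-unit X/Z cells, typing them by actor tag.
; Helpers provide clamped directional neighbor lookup, wall collision checks, and pellet consumption that deactivates the cell and hides its actor.
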(event `self.ReceiveBeginPlay`
  (`self.InitializeGrid`)
  (`self.ProcessBatchAndFillGrid`))

(fn `CheckCollision`
  (params (Position :type "IntPoint Structure"))
  (returns (IsColliding :type Boolean))
  (bind _gridcell (`self.GetCell` Position_X Position_Y))
  (bind _celltype (break `/Game/Blueprints/BPS_GridCell` _gridcell))
  (return (or (`|EnumEquality` _celltype "NewEnumerator4") (`|EnumEquality` _celltype "NewEnumerator5"))))

(fn `CheckPellet`
  (params (IntPointPosition :type "IntPoint Structure"))
  (returns (AtePellet :type Boolean))
  (bind (_row _column) (`self.TransformIntPoint` IntPointPosition))
  (bind _gridcell (`self.GetCell` _row _column))
  (bind (_celltype _isactive _actorref) (break `/Game/Blueprints/BPS_GridCell` _gridcell))
  (if (and (`|EnumEquality` _celltype "NewEnumerator1") _isactive)
    (`self.SetCell` _row _column (make `/Game/Blueprints/BPS_GridCell` _celltype false _actorref))
    (`self.SetActorHiddenInGame` _actorref true)
    (return true)
    (else
      (return false))))

(fn `CheckTag`
  (params (ActorRef :type "Actor Object Reference"))
  (returns (CellType :type "/Game/Blueprints/E_GridCellType Enum"))
  (locals (GridCellType :type "/Game/Blueprints/E_GridCellType Enum"))
  ;[1 1 1] Set Cell Type depending on the Actor's Tag
  (if (`self.ActorHasTag` ActorRef "PowerPellet")
    (set `local.GridCellType` "NewEnumerator2")
    (elif (`self.ActorHasTag` ActorRef "Pellet")
      (set `local.GridCellType` "NewEnumerator1")
      (elif (`self.ActorHasTag` ActorRef "StaticWall")
        (set `local.GridCellType` "NewEnumerator4")
        (elif (`self.ActorHasTag` ActorRef "MovingWall")
          (set `local.GridCellType` "NewEnumerator5")
          (else
            (set `local.GridCellType` "NewEnumerator0"))))))
  (return (`local.GridCellType`)))

(fn `GetCell`
  (params (Row :type Integer) (Column :type Integer))
  (returns (GridCell :type "/Game/Blueprints/BPS_GridCell Structure"))
  (bind _index (`self.GetGridIndex` Row Column))
  (return (`|GetArrayItem` (`self.GridArray`) _index)))

(fn `GetGridIndex`
  (params (Row :type Integer) (Column :type Integer))
  (returns (Index :type Integer))
  ;[1 1 1] Get the Grid Cell Index (Row * Columns + Column)
  (return (+ (* Row (`self.Columns`)) Column)))

(fn `GetNeighborCell`
  (params (Row :type Integer) (Column :type Integer) (Direction :type "/Game/Blueprints/E_GridDirection Enum" :default "NewEnumerator0") (Distance :type Integer))
  (returns (NeighborCell :type "/Game/Blueprints/BPS_GridCell Structure"))
  (bind (_neighborrow _neighborcolumn) (`self.GetNeighborCoordinates` Row Column Direction Distance))
  (bind _gridcell (`self.GetCell` _neighborrow _neighborcolumn))
  (return _gridcell))

(fn `GetNeighborCoordinates`
  (params (Row :type Integer) (Column :type Integer) (Direction :type "/Game/Blueprints/E_GridDirection Enum" :default "NewEnumerator0") (Distance :type Integer))
  (returns (NeighborRow :type Integer) (NeighborColumn :type Integer))
  (locals (TempColumn :type Integer) (TempRow :type Integer))
  ;[1 1 1] Apply Direction Math
  (switch `/Game/Blueprints/E_GridDirection` Direction
    (:`NewEnumerator0`
      ;[1 1 1] Set Rows
      (set `local.TempRow` (- Row Distance))
      (set `local.TempColumn` Column :!label _label))
    (:`NewEnumerator1`
      (set `local.TempRow` (+ Row Distance))
      (goto _label))
    (:`NewEnumerator2`
      (set `local.TempColumn` (- Column Distance))
      (set `local.TempRow` Row :!label _label_2))
    (:`NewEnumerator3`
      (set `local.TempColumn` (+ Column Distance))
      (goto _label_2)))
  (return (`KismetMathLibrary.Clamp` (`local.TempRow`) 0 (- (`self.Rows`) 1)) (`KismetMathLibrary.Clamp` (`local.TempColumn`) 0 (- (`self.Columns`) 1))))

(fn `InitializeGrid`
  (`KismetArrayLibrary.Array_Clear` (`self.GridArray`))
  (for _ (range (* (`self.Rows`) (`self.Columns`)))
    (`KismetArrayLibrary.Array_Add` (`self.GridArray`) (make `/Game/Blueprints/BPS_GridCell` "NewEnumerator0" true))))

(fn `PrintGrid`
  (for _array_element (`self.GridArray`)
    (bind (_celltype _isactive _actorref) (break `/Game/Blueprints/BPS_GridCell` _array_element))
    (`KismetSystemLibrary.PrintString` (`KismetStringLibrary.Concat_StrStr` "Actor " (`KismetSystemLibrary.GetDisplayName` _actorref) " with Cell Type " (`|GetEnumeratorNameAsString` _celltype)))))

(fn `ProcessBatchAndFillGrid`
  (bind _outactors (`GameplayStatics.GetAllActorsOfClass` "/Script/Paper2D.PaperSpriteActor"))
  (for _array_element _outactors
    (bind _returnvalue (`self.GetComponentByClass` _array_element "/Game/Blueprints/BP_GridComponent.BP_GridComponent_C"))
    ;[1 1 1] Check if the Actor has a BP_GridComponent; add one if not
    (if (`KismetSystemLibrary.IsValid` _returnvalue)
      ;[1 1 1] Create the Grid Cell Struct
      (bind _output_get (set `/Game/Blueprints/BP_GridComponent.GridPosition` (make `IntPoint` (`KismetMathLibrary.Clamp` (`KismetMathLibrary.FFloor` (/ (.x (`self.K2_GetActorLocation` _array_element)) 16.0)) 0 27) (`KismetMathLibrary.Clamp` (`KismetMathLibrary.FFloor` (/ (.z (`self.K2_GetActorLocation` _array_element)) 16.0)) 0 30)) _returnvalue))
      (bind _celltype (`self.CheckTag` _array_element))
      (bind _output_get_2 (set `/Game/Blueprints/BP_GridComponent.GridCell` (make `/Game/Blueprints/BPS_GridCell` _celltype (`.IsActive_5_DE00E2B1419E7C3ED20A8F8147D2EB1C` (break `/Game/Blueprints/BPS_GridCell` (`/Game/Blueprints/BP_GridComponent.GridCell` _returnvalue))) _array_element) _returnvalue))
      (bind (_x _y) (break `IntPoint` _output_get))
      (`self.SetCell` _x _y _output_get_2)
      (bind _index (`self.GetGridIndex` _x _y))
      (`KismetSystemLibrary.LogString` (`KismetStringLibrary.Concat_StrStr` "Actor at index " (`KismetStringLibrary.Conv_IntToString` _index) ": " (`KismetSystemLibrary.GetDisplayName` _array_element))))))

(fn `SetCell`
  (params (Row :type Integer) (Column :type Integer) (NewCellType :type "/Game/Blueprints/BPS_GridCell Structure"))
  ;[1 1 1] Set the Cell Type at a specified index
  (bind _index (`self.GetGridIndex` Row Column))
  (`KismetArrayLibrary.Array_Set` (`self.GridArray`) _index NewCellType))

(fn `TransformIntPoint`
  (params (IntPointPosition :type "IntPoint Structure"))
  (returns (Row :type Integer) (Column :type Integer))
  (bind (_x _y) (break `IntPoint` IntPointPosition))
  (return _x _y))

(fn `UserConstructionScript`)
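; BP_Ghost is a grid-moving ghost that steers toward a target grid position.
; Each Tick, it sets the grid character component's move direction from GetCardinalVectorTowardsTarget.
; That function rounds the angle between the target offset and +X to 90 degrees, then converts it to an integer vector.
; Because Acos yields an unsigned angle, the result never points toward -Y, and TargetGridPosition is not set here.
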(event `self.ReceiveTick`
  (params (DeltaSeconds :type "Float (single-precision)"))
  (bind _cardinalvector (`self.GetCardinalVectorTowardsTarget`))
  (set `/Game/Blueprints/BP_GridCharacterComponent.GridMoveDirection` _cardinalvector (`self.BP_GridCharacterComponent`)))

(fn `GetCardinalVectorTowardsTarget`
  (returns (CardinalVector :type "IntPoint Structure"))
  (bind _returnvalue (/ (`KismetMathLibrary.GetPI`) 2.0))
  (bind _returnvalue_2 (* (`KismetMathLibrary.Round` (/ (`KismetMathLibrary.Acos` (`KismetMathLibrary.DotProduct2D` (`KismetMathLibrary.Normal2D` (- (`self.TargetGridPosition`) (`/Game/Blueprints/BP_GridCharacterComponent.GridPosition` (`self.BP_GridCharacterComponent`)))) (1.0 0.0))) _returnvalue)) _returnvalue))
  (return (make `IntPoint` (`KismetMathLibrary.Round` (`KismetMathLibrary.Cos` _returnvalue_2)) (`KismetMathLibrary.Round` (`KismetMathLibrary.Sin` _returnvalue_2)))))

(fn `UserConstructionScript`)
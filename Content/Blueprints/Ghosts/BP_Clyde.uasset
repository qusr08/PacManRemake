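; BP_Clyde is the Clyde ghost, a child Blueprint that chooses its grid target based on proximity to Pac-Man.
; Each Tick it compares squared 2D distance between both grid positions, targeting Pac-Man's cell within eight cells and otherwise the bottom-left corner at the grid origin.
; It then calls the parent Tick, leaving all other behavior to the parent class.
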(event `self.ReceiveTick`
  (params (DeltaSeconds :type "Float (single-precision)"))
  (bind _gridposition (`/Game/Blueprints/BP_GridCharacterComponent.GridPosition` (`/Game/Blueprints/BP_PacMan.BP_GridCharacterComponent` (`self.PacManReference`))))
  (if (<= (`KismetMathLibrary.DistanceSquared2D` (`KismetMathLibrary.Conv_IntPointToVector2D` _gridposition) (`KismetMathLibrary.Conv_IntPointToVector2D` (`/Game/Blueprints/BP_GridCharacterComponent.GridPosition` (`self.BP_GridCharacterComponent`)))) 64.0)
    (set `self.TargetGridPosition` _gridposition)
    (else
      (set `self.TargetGridPosition` (make `IntPoint` 0))))
  (`parent.ReceiveTick` DeltaSeconds))

(fn `UserConstructionScript`
  (`parent.UserConstructionScript`))
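; BP_Inky is the Inky ghost in a grid-based Pac-Man game, computing the grid tile it targets each tick.
; It takes a pivot two tiles ahead of Pac-Man along his move direction and mirrors Blinky's grid position through it.
; The result becomes TargetGridPosition before the parent ghost's Tick runs; the construction script only calls the parent.
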(event `self.ReceiveTick`
  (params (DeltaSeconds :type "Float (single-precision)"))
  (bind _bp_gridcharactercomponent (`/Game/Blueprints/BP_PacMan.BP_GridCharacterComponent` (`self.PacManReference`)))
  (bind _returnvalue (+ (`/Game/Blueprints/BP_GridCharacterComponent.GridPosition` _bp_gridcharactercomponent) (* (`/Game/Blueprints/BP_GridCharacterComponent.GridMoveDirection` _bp_gridcharactercomponent) (make `IntPoint` 2 2))))
  (set `self.TargetGridPosition` (+ _returnvalue (- _returnvalue (`/Game/Blueprints/BP_GridCharacterComponent.GridPosition` (`/Game/Blueprints/Ghosts/BP_Ghost.BP_GridCharacterComponent` (`self.Blinky Reference`))))))
  (`parent.ReceiveTick` DeltaSeconds))

(fn `UserConstructionScript`
  (`parent.UserConstructionScript`))
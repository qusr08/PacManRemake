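; Pac-Man ghost actor that steers its grid character component toward a chase target, scatter position or ghost house, depending on its state.
; Each tick picks the unblocked neighboring cell closest to that target, reversing only when no other direction is found.
; A timer switches Chase to Scatter; no other transitions exist here, and SetGhostState only stores the state.
; The Pac-Man reference is cached but unused, and TargetGridPosition is never set here.
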(event `self.ReceiveBeginPlay`
  (bind _returnvalue (`GameplayStatics.GetActorOfClass` "/Game/Blueprints/BP_PacMan.BP_PacMan_C"))
  (set `self.PacManReference` _returnvalue))

(event `self.ReceiveTick`
  (params (DeltaSeconds :type "Float (single-precision)"))
  (set `self.GhostStateTimer` (+ DeltaSeconds (`self.GhostStateTimer`)))
  (switch `/Game/Blueprints/Ghosts/E_GhostState` (`self.GhostState`)
    (:`NewEnumerator0`
      ;[1 1 1] Handle ghost movement in chase mode
      (if (>= (`self.GhostStateTimer`) (`self.ChaseTime`))
        (`self.SetGhostState` "NewEnumerator1"))
      (bind _cardinalvector (`self.GetCardinalVectorTowardsTarget` (`self.TargetGridPosition`)))
      (set `/Game/Blueprints/BP_GridCharacterComponent.GridTryMoveDirection` _cardinalvector (`self.BP_GridCharacterComponent`)))
    (:`NewEnumerator1`
      ;[1 1 1] Handle ghost movement in scatter mode
      (bind _cardinalvector_2 (`self.GetCardinalVectorTowardsTarget` (`self.ScatterGridPosition`)))
      (set `/Game/Blueprints/BP_GridCharacterComponent.GridTryMoveDirection` _cardinalvector_2 (`self.BP_GridCharacterComponent`)))
    (:`NewEnumerator3`
      ;[1 1 1] Handle ghost movement in return mode
      (bind _cardinalvector_3 (`self.GetCardinalVectorTowardsTarget` (`self.GhostHouseGridPosition`)))
      (set `/Game/Blueprints/BP_GridCharacterComponent.GridTryMoveDirection` _cardinalvector_3 (`self.BP_GridCharacterComponent`)))))

(fn `GetCardinalVectorTowardsTarget`
  (params (TargetPosition :type "IntPoint Structure"))
  (returns (CardinalVector :type "IntPoint Structure"))
  (locals (BestMoveDirection :type "IntPoint Structure") (LowestMoveDistance :type "Float (double-precision)" :default 9999999.0))
  (bind _bp_gridcharactercomponent (`self.BP_GridCharacterComponent`))
  (bind _bp_gridcharactercomponent_2 (`self.BP_GridCharacterComponent`))
  (bind _bp_gridcharactercomponent_3 (`self.BP_GridCharacterComponent`))
  (for _array_element (`|MakeArray` (`KismetMathLibrary.IntPoint_Up`) (`KismetMathLibrary.IntPoint_Right`) (`KismetMathLibrary.IntPoint_Down`) (`KismetMathLibrary.IntPoint_Left`))
    (bind _returnvalue (+ (`/Game/Blueprints/BP_GridCharacterComponent.GridPosition` _bp_gridcharactercomponent) _array_element))
    ;[1 1 1] Skip directions that collide with the grid
    (bind _iscolliding (`/Game/Blueprints/BP_Grid.CheckCollision` (`/Game/Blueprints/BP_GridCharacterComponent.GridReference` _bp_gridcharactercomponent) _returnvalue))
    (if (not _iscolliding)
      ;[1 1 1] Skip the direction if it is directly opposite the current move direction
      (if (not (`/Game/Blueprints/BP_GridCharacterComponent.IsIntPointEqual` _bp_gridcharactercomponent_3 (`/Game/Blueprints/BP_GridCharacterComponent.GetOppositeIntPoint` _bp_gridcharactercomponent_3 (`/Game/Blueprints/BP_GridCharacterComponent.GridMoveDirection` _bp_gridcharactercomponent_3)) _array_element))
        (bind _returnvalue_2 (`KismetMathLibrary.DistanceSquared2D` (`KismetMathLibrary.Conv_IntPointToVector2D` TargetPosition) (`KismetMathLibrary.Conv_IntPointToVector2D` _returnvalue)))
        ;[1 1 1] Check to see if the current direction movement has the lowest distance to the target
        (if (< _returnvalue_2 (`local.LowestMoveDistance`))
          (set `local.BestMoveDirection` _array_element)
          (set `local.LowestMoveDistance` _returnvalue_2)))))
  ;[1 1 1] If there was no best movement direction found, then the only direction to move should be the opposite direction to where it is currently moving
  (if (`/Game/Blueprints/BP_GridCharacterComponent.IsIntPointEqual` _bp_gridcharactercomponent_2 (`local.BestMoveDirection`) (make `IntPoint` 0))
    (set `local.BestMoveDirection` (`/Game/Blueprints/BP_GridCharacterComponent.GetOppositeIntPoint` _bp_gridcharactercomponent_2 (`/Game/Blueprints/BP_GridCharacterComponent.GridMoveDirection` _bp_gridcharactercomponent_2))))
  (return (`local.BestMoveDirection`)))

(fn `SetGhostState`
  (params (GhostState :type "/Game/Blueprints/Ghosts/E_GhostState Enum" :default "NewEnumerator0"))
  (bind _output_get (set `self.GhostState` GhostState))
  (switch `/Game/Blueprints/Ghosts/E_GhostState` _output_get))

(fn `UserConstructionScript`)
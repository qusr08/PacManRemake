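; BP_PacMan is the player-controlled Pac-Man, steered in four directions on a grid.
; On BeginPlay it adds the INC_PlayerInputMapping Enhanced Input context to player controller 0's local player subsystem.
; Each IA_Move action writes a unit direction to GridTryMoveDirection on BPGridCharacterComponent, leaving the movement itself to that component.
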(event `self.ReceiveBeginPlay`
  (bind _returnvalue (pcsubsystem `EnhancedInputLocalPlayerSubsystem` (`GameplayStatics.GetPlayerController` 0)))
  (`/Engine/EditorBlueprintResources/StandardMacros.IsValid` _returnvalue
    (:`Is Valid`
      (`EnhancedInputSubsystemInterface.AddMappingContext` _returnvalue "/Game/Input/INC_PlayerInputMapping.INC_PlayerInputMapping" 0 (struct)))))

(event `EnhancedInput|/Game/Input/IA_Move_Up`
  (params (ActionValue :type "Float (double-precision)") (ElapsedSeconds :type "Float (double-precision)") (TriggeredSeconds :type "Float (double-precision)") (InputAction :type "InputAction Object Reference" :default "/Game/Input/IA_Move_Up.IA_Move_Up"))
  (:`Triggered`
    (set `/Game/Blueprints/BP_GridCharacterComponent.GridTryMoveDirection` (make `IntPoint` 0 1) (`self.BP_GridCharacterComponent`))))

(event `EnhancedInput|/Game/Input/IA_Move_Right`
  (params (ActionValue :type "Float (double-precision)") (ElapsedSeconds :type "Float (double-precision)") (TriggeredSeconds :type "Float (double-precision)") (InputAction :type "InputAction Object Reference" :default "/Game/Input/IA_Move_Right.IA_Move_Right"))
  (:`Triggered`
    (set `/Game/Blueprints/BP_GridCharacterComponent.GridTryMoveDirection` (make `IntPoint` 1) (`self.BP_GridCharacterComponent`))))

(event `EnhancedInput|/Game/Input/IA_Move_Down`
  (params (ActionValue :type "Float (double-precision)") (ElapsedSeconds :type "Float (double-precision)") (TriggeredSeconds :type "Float (double-precision)") (InputAction :type "InputAction Object Reference" :default "/Game/Input/IA_Move_Down.IA_Move_Down"))
  (:`Triggered`
    (set `/Game/Blueprints/BP_GridCharacterComponent.GridTryMoveDirection` (make `IntPoint` 0 -1) (`self.BP_GridCharacterComponent`))))

(event `EnhancedInput|/Game/Input/IA_Move_Left`
  (params (ActionValue :type "Float (double-precision)") (ElapsedSeconds :type "Float (double-precision)") (TriggeredSeconds :type "Float (double-precision)") (InputAction :type "InputAction Object Reference" :default "/Game/Input/IA_Move_Left.IA_Move_Left"))
  (:`Triggered`
    (set `/Game/Blueprints/BP_GridCharacterComponent.GridTryMoveDirection` (make `IntPoint` -1) (`self.BP_GridCharacterComponent`))))

(fn `UserConstructionScript`)
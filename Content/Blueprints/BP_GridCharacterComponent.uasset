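; Actor component that moves its owning Paper2D character cell by cell across a BP_Grid in the XZ plane.
; Whenever idle, Tick tries a step along GridMoveDirection, rejecting two blocking cell types and clearing the direction when blocked.
; An accepted step updates the grid position, restarts a countdown timer that linearly interpolates the owner between cells, and selects the directional flipbook.
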(event `self.ReceiveBeginPlay`
  (bind _gridworldsize (`self.GridWorldSize`))
  (bind (_gridposition_x _gridposition_y) (break `IntPoint` (`self.GridPosition`)))
  (bind _returnvalue (`GameplayStatics.GetActorOfClass` "/Game/Blueprints/BP_Grid.BP_Grid_C"))
  (set `self.Grid Reference` _returnvalue) ; Set the grid reference on start
  (bind _output_get (set `self.FlipbookReference` (`Actor.GetComponentByClass` (`self.GetOwner`) "/Script/Paper2D.PaperFlipbookComponent")))
  (`PaperFlipbookComponent.SetFlipbook` _output_get (`self.MoveRight`)) ; Set the initial flipbook sprite of the character
  (bind _output_get_2 (set `self.FromLocation` (`KismetMathLibrary.MakeVector` (* _gridposition_x _gridworldsize) 0.0 (* _gridposition_y _gridworldsize))))
  (set `self.ToLocation` (`KismetMathLibrary.MakeVector` (.x _output_get_2) 0.0 (.z _output_get_2))))

(event `self.ReceiveTick`
  (params (DeltaSeconds :type "Float (single-precision)"))
  (if (`self.IsAnimatingMovement`)
    (set `self.GridMoveTimer` (- (`self.GridMoveTimer`) DeltaSeconds))
    (`Actor.K2_SetActorLocation` (`self.GetOwner`) (`self.GetLerpLocation`) false false)
    (else
      (set `self.FromLocation` (`self.ToLocation`))
      (`self.Try Grid Movement`))))

(fn `GetLerpLocation`
  (returns (LerpLocation :type "Vector Structure"))
  (return (`KismetMathLibrary.VLerp` (`self.FromLocation`) (`self.ToLocation`) (- 1.0 (/ (`self.GridMoveTimer`) (`self.GridMoveTime`))))))

(fn `IsAnimatingMovement`
  (returns (IsAnimatingMovement :type Boolean))
  (return (> (`self.GridMoveTimer`) 0.0)))

(fn `SetFlipbookFromDirection`
  (params (Direction :type "IntPoint Structure"))
  (locals (FlipbookIndex :type Integer))
  (if (> Direction_Y 0)
    (set `local.FlipbookIndex` 0)
    (elif (< Direction_Y 0)
      (set `local.FlipbookIndex` 2)
      (elif (< Direction_X 0)
        (set `local.FlipbookIndex` 3)
        (else
          (set `local.FlipbookIndex` 1)))))
  (`PaperFlipbookComponent.SetFlipbook` (`self.FlipbookReference`) (select `int` (`local.FlipbookIndex`) :`0` (`self.MoveUp`) :`1` (`self.MoveRight`) :`2` (`self.MoveDown`) :`3` (`self.MoveLeft`))))

(fn `Try Grid Movement`
  (returns (Moved :type Boolean))
  (bind _gridworldsize (`self.GridWorldSize`))
  (bind _grid_reference (`self.Grid Reference`))
  (bind (_row _column) (`/Game/Blueprints/BP_Grid.TransformIntPoint` _grid_reference (+ (`self.GridMoveDirection`) (`self.GridPosition`))))
  (bind _gridcell (`/Game/Blueprints/BP_Grid.GetCell` _grid_reference _row _column))
  (bind _celltype (break `/Game/Blueprints/BPS_GridCell` _gridcell))
  (if (not (or (`|EnumEquality` _celltype "NewEnumerator4") (`|EnumEquality` _celltype "NewEnumerator5")))
    (bind _output_get (set `self.GridPosition` (+ (`self.GridMoveDirection`) (`self.GridPosition`)))) ; Set the new grid position based on the movement direction
    (set `self.ToLocation` (`KismetMathLibrary.MakeVector` (* (break `IntPoint` _output_get) _gridworldsize) 0.0 (* (`.Y` (break `IntPoint` _output_get)) _gridworldsize))) ; Get the to location position so the character\nknows where in world space it is going to move to
    (set `self.GridMoveTimer` (`self.GridMoveTime`)) ; Reset the move timer so the character can\nstart moving
    (`self.SetFlipbookFromDirection` (`self.GridMoveDirection`)) ; Update the flipbook sprite based on the move direction
    (return true)
    (else
      (set `self.GridMoveDirection` (make `IntPoint` 0)))))
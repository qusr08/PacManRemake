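; BP_GridComponent manages a grid cell's actor, blinking it as a timed transition into a spawned or despawned state.
; While blinking, Tick accumulates time and toggles the cell actor's visibility using thresholds on an absolute sine wave.
; When the duration ends, it sets final visibility from IsSpawning and writes the cell's active state back to the Grid.
; SetVisibility passes its Visible flag straight into the owner's hidden-in-game setting, so true hides it.
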(event `self.ReceiveTick`
  (params (DeltaSeconds :type "Float (single-precision)"))
  (bind _isspawning (`self.isSpawning`))
  (bind _grid (`self.Grid`))
  (bind (_celltype _isactive _actorref) (break `/Game/Blueprints/BPS_GridCell` (`self.GridCell`)))
  (if (`self.isBlinking`)
    ;[1 1 1] If spawning, update the blink time
    (bind _output_get (set `self.BlinkTimeElapsed` (+ DeltaSeconds (`self.BlinkTimeElapsed`))))
    ;[1 1 1] Check if the blinking duration has ended
    (if (>= _output_get (`self.BlinkDuration`))
      ;[1 1 1] Stop blinking and enable the wall
      (set `self.isBlinking` false)
      (`Actor.SetActorHiddenInGame` (`.ActorRef_8_8561F30E44B9EBEF63EE34AD8B14F00C` (break `/Game/Blueprints/BPS_GridCell` (`self.GridCell`))) (not _isspawning))
      (bind _structout (setmembers `/Game/Blueprints/BPS_GridCell` :`StructRef` (`self.GridCell`) :`IsActive` _isspawning))
      (bind (_row _column) (`/Game/Blueprints/BP_Grid.TransformIntPoint` _grid (`self.GridPosition`)))
      (`/Game/Blueprints/BP_Grid.SetCell` _grid _row _column _structout)
      (set `self.BlinkTimeElapsed` 0.0)
      (else
        (bind _returnvalue (`KismetMathLibrary.Abs` (`KismetMathLibrary.Sin` (* _output_get (`self.BlinkFrequency`)))))
        ;[1 1 1] Check if the Actor should be Hidden (Blink)
        (if (>= _returnvalue 0.8)
          (`Actor.SetActorHiddenInGame` _actorref true)
          (elif (<= _returnvalue 0.2)
            (`Actor.SetActorHiddenInGame` _actorref false)))))))

(fn `SetVisibility`
  (params (Visible :type Boolean))
  ;[1 1 1] Set whether or not the Actor is visible in game
  (`Actor.SetActorHiddenInGame` (`self.GetOwner`) Visible))